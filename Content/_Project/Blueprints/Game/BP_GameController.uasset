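; BP_GameController is a player controller that provides helper functions for managing Enhanced Input mapping contexts.
; AddInputContext adds a context at a given priority only if the local player's subsystem lacks it, and RemoveInputContext removes one only if present.
; The event graph and construction script are empty, so neither function is called within this Blueprint.
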(fn `AddInputContext`
  (params (MappingContext :type "InputMappingContext Object Reference") (Priority :type Integer))
  (bind _returnvalue (pcsubsystem `EnhancedInputLocalPlayerSubsystem` self))
  (if (not (`.ReturnValue` (`EnhancedInputSubsystemInterface.HasMappingContext` _returnvalue MappingContext)))
    (`EnhancedInputSubsystemInterface.AddMappingContext` _returnvalue MappingContext Priority (struct))))

(fn `RemoveInputContext`
  (params (MappingContext :type "InputMappingContext Object Reference"))
  (bind _returnvalue (pcsubsystem `EnhancedInputLocalPlayerSubsystem` self))
  (if (`.ReturnValue` (`EnhancedInputSubsystemInterface.HasMappingContext` _returnvalue MappingContext))
    (`EnhancedInputSubsystemInterface.RemoveMappingContext` _returnvalue MappingContext (struct))))

(fn `UserConstructionScript`)