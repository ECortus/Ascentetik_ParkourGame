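; Level path actor that measures how far a location, treated as the player's, has progressed along one or more splines.
; On BeginPlay it gathers its spline components and stores their average length as the path length.
; GetCompletedLengthByLocation flattens the location to the actor's height and finds each spline's closest point.
; It blends completed fraction and remaining distance with Gaussian weights relative to the nearest spline, smoothing transitions between branches.
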(event `self.ReceiveBeginPlay`
  (`KismetArrayLibrary.Array_Clear` (`self.SplineCollection`))
  (for _array_element (`self.K2_GetComponentsByClass` self "/Script/Engine.ActorComponent")
    (bind _asspline_component (cast `SplineComponent` _array_element))
    (`KismetArrayLibrary.Array_Add` (`self.SplineCollection`) _asspline_component))
  (`self.SetPathLength`))

(fn `GetCompletedLengthByLocation`
  (params (Location :type "Vector Structure (by ref)"))
  (returns (Fraction :type "Float (double-precision)") (Remaining :type "Float (double-precision)"))
  (locals (MinDistance :type "Float (double-precision)") (SplineDistances :type "Array of Float (double-precision)") (SplineFractions :type "Array of Float (double-precision)") (SplineRemainings :type "Array of Float (double-precision)") (PlayerLocation :type "Vector Structure") (PlayerLocationNormalized :type "Vector Structure") (SumW :type "Float (double-precision)") (SumF :type "Float (double-precision)") (SumR :type "Float (double-precision)") (W_i :type "Float (double-precision)"))
  (bind _w_i (`local.W_i`))
  (bind _sumw (`local.SumW`))
  (bind _playerlocationnormalized (`local.PlayerLocationNormalized`))
  (bind (_returnvalue_x _returnvalue_y _returnvalue_z) (`KismetMathLibrary.BreakVector` (`self.K2_GetActorLocation` self)))
  (bind _output_get (set `local.PlayerLocation` Location))
  (set `local.PlayerLocationNormalized` (`KismetMathLibrary.MakeVector` (.x _output_get) (.y _output_get) _returnvalue_z))
  (`KismetArrayLibrary.Array_Clear` (`local.SplineDistances`))
  (`KismetArrayLibrary.Array_Clear` (`local.SplineFractions`))
  (`KismetArrayLibrary.Array_Clear` (`local.SplineRemainings`))
  (set `local.MinDistance` 999999.0)
  (for _array_element (`self.SplineCollection`)
    (bind _returnvalue (`SplineComponent.FindLocationClosestToWorldLocation` _array_element _playerlocationnormalized "World"))
    (`KismetArrayLibrary.Array_Add` (`local.SplineDistances`) (`KismetMathLibrary.Vector_Distance` _playerlocationnormalized _returnvalue))
    (bind _returnvalue_2 (`SplineComponent.GetDistanceAlongSplineAtLocation` _array_element _returnvalue "World"))
    (bind _returnvalue_3 (`SplineComponent.GetSplineLength` _array_element))
    (`KismetArrayLibrary.Array_Add` (`local.SplineFractions`) (/ _returnvalue_2 _returnvalue_3))
    (`KismetArrayLibrary.Array_Add` (`local.SplineRemainings`) (- _returnvalue_3 _returnvalue_2)))
  (set `local.MinDistance` (`.MinValue` (`KismetMathLibrary.MinOfFloatArray` (`local.SplineDistances`))))
  (set `local.SumW` 0.0)
  (set `local.SumF` 0.0)
  (set `local.SumR` 0.0)
  (for (_ _array_index) (`self.SplineCollection`)
    (set `local.W_i` (`KismetMathLibrary.Exp` (* (`KismetMathLibrary.Square` (/ (- (`|GetArrayItem` (`local.SplineDistances`) _array_index) (`local.MinDistance`)) 300.0)) -1.0)))
    (set `local.SumW` (+ (`local.SumW`) _w_i))
    (set `local.SumF` (+ (`local.SumF`) (* _w_i (`|GetArrayItem` (`local.SplineFractions`) _array_index))))
    (set `local.SumR` (+ (`local.SumR`) (* _w_i (`|GetArrayItem` (`local.SplineRemainings`) _array_index)))))
  (bind _output_get_2 (set `self.PathFraction` (/ (`local.SumF`) _sumw)))
  (bind _output_get_3 (set `self.PathRemaining` (/ (`local.SumR`) _sumw)))
  (return _output_get_2 _output_get_3))

(fn `GetPathLength`
  (returns (Length :type "Float (double-precision)"))
  (return (`self.PathLength`)))

(fn `SetPathLength`
  (locals (SumPathsLength :type "Float (double-precision)"))
  (bind _splinecollection (`self.SplineCollection`))
  (set `local.SumPathsLength` 0.0)
  (for _array_element _splinecollection
    (set `local.SumPathsLength` (+ (`local.SumPathsLength`) (`SplineComponent.GetSplineLength` _array_element))))
  (set `self.PathLength` (/ (`local.SumPathsLength`) (`KismetArrayLibrary.Array_Length` _splinecollection))))

(fn `UserConstructionScript`)