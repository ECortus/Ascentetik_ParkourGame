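; Footstep component for BP_Character that attaches the character's left and right foot components to mesh sockets and plays positional footstep sounds.
; Begin Play disables its tick; when ticking, it plays one fixed sound whenever a foot socket drops below a root-relative height, printing that height for debugging.
; It stores the root's previous location for velocity-based volume, but that mapping is left unwired, as is a foot-angle check.
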(event `self.ReceiveBeginPlay`
  ; Begin Play
  (bind _asbp_character (cast `/Game/_Project/Blueprints/Player/Character/BP_Character` (`self.GetOwner`)))
  (set `self.Owner` _asbp_character)
  (set `self.Mesh` (`Character.Mesh` _asbp_character))
  (set `self.FootLeft` (`/Game/_Project/Blueprints/Player/Character/BP_Character.FootLeft` _asbp_character))
  (set `self.FootRight` (`/Game/_Project/Blueprints/Player/Character/BP_Character.FootRight` _asbp_character))
  (`SceneComponent.K2_AttachToComponent` (`self.FootLeft`) (`self.Mesh`) (`self.LeftSocketName`) "SnapToTarget" "SnapToTarget" "SnapToTarget" true)
  (`SceneComponent.K2_AttachToComponent` (`self.FootRight`) (`self.Mesh`) (`self.RightSocketName`) "SnapToTarget" "SnapToTarget" "SnapToTarget" true)
  (`self.SetComponentTickEnabled` false))

(event `self.ReceiveTick`
  (params (DeltaSeconds :type "Float (single-precision)"))
  ; Tick
  (`|ExecutionSequence`
    (:`then_0`
      (`self.UpdateFoot` (`self.LeftSocketName`) (`self.FootLeft`) DeltaSeconds))
    (:`then_1`
      (`self.UpdateFoot` (`self.RightSocketName`) (`self.FootRight`) DeltaSeconds))))

(fn `SetRootPreviousLocation`
  (set `self.RootPreviousLocation` (`SceneComponent.K2_GetComponentLocation` (`Actor.RootComponent` (`self.Owner`))))
  (return))

(fn `ShouldPlayFootstep`
  (params (`Socket Name` :type Name) (Foot :type "AudioComponent Object Reference"))
  (returns (Play :type Boolean))
  (bind _owner (`self.Owner`))
  (bind (_returnvalue_x _returnvalue_y _returnvalue_z) (`KismetMathLibrary.BreakVector` (`SceneComponent.GetSocketLocation` (`Character.Mesh` _owner) (`local.Socket Name`))))
  (bind (_returnvalue_x_2 _returnvalue_y_2 _returnvalue_z_2) (`KismetMathLibrary.BreakVector` (`SceneComponent.K2_GetComponentLocation` (`Actor.RootComponent` _owner))))
  (bind _returnvalue (- _returnvalue_z_2 78.0))
  (`KismetSystemLibrary.PrintString` (`KismetStringLibrary.Concat_StrStr` (`KismetStringLibrary.Conv_NameToString` `Socket Name`) ", difference:  " (`KismetStringLibrary.Conv_DoubleToString` (- _returnvalue_z _returnvalue))))
  (return (or (< _returnvalue_z _returnvalue) false)))

(fn `UpdateFootstepSound`
  (params (Foot :type "AudioComponent Object Reference"))
  (returns (`Footstep Sound` :type "SoundBase Object Reference"))
  (bind _output_get (set `self.FootStep_Sound` "/Game/_Project/Audio/Gameplay/MSP_Footsteps0.MSP_Footsteps0"))
  (return _output_get))