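; Player controller that runs a spline-route run: sets up input and HUD, spawns and possesses the player, and handles pause, win, lose and restart.
; A looping timer measures completion along the first tagged BP_SplinePath, while Tick accumulates run time.
; Win and lose pause the game, show an end screen and store the best completion and time per difficulty in BP_GameInstance.
; The per-mode completion update is disabled, so progress always uses spline percentage.
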(event `self.ReceiveBeginPlay`)

(event `InitializeController`
  (bind _asbp_game_instance (cast `/Game/_Project/Blueprints/Game/BP_GameInstance` (`GameplayStatics.GetGameInstance`)))
  (bind _output_get (set `self.GameInstance` _asbp_game_instance))
  (`|ExecutionSequence`
    (:`then_0`
      (switch `EGameDifficulty` (`/Game/_Project/Blueprints/Game/BP_GameInstance.SelectedDifficulty` _output_get)
        (:`Easy`
          (set `self.CompletionType` "NewEnumerator0" :!label _label))
        (:`Regular`
          (goto _label))
        (:`Hard`
          (goto _label))
        (:`Endless`
          (set `self.CompletionType` "NewEnumerator1"))))
    (:`then_1`
      (`|ExecutionSequence`
        (:`then_0`
          (`self.AddInputContext` "/Game/_Project/Blueprints/Player/Input/UI/IMC_UI.IMC_UI" 1)
          (`self.AddInputContext` "/Game/_Project/Blueprints/Player/Input/IMC_Gameplay.IMC_Gameplay" 2))
        (:`then_1`
          (bind _returnvalue (`|CreateWidget` "/Game/_Project/UI/WBP_HUD.WBP_HUD_C"))
          (bind _output_get_2 (set `self.HUDWidget` _returnvalue))
          (`UserWidget.AddToViewport` _output_get_2 -1))
        (:`then_2`
          (`|ExecutionSequence`
            (:`then_0`
              (bind _outactors (`GameplayStatics.GetAllActorsWithTag` "Spline_Path"))
              (set `self.PathSpline` (`|MakeArray`))
              (for _array_element _outactors
                (`/Engine/EditorBlueprintResources/StandardMacros.IsValid` _array_element
                  (:`Is Valid`
                    (bind _asbp_spline_path (cast `/Game/_Project/Blueprints/LevelDesign/Elements/BP_SplinePath` _array_element))
                    (`KismetArrayLibrary.Array_Add` (`self.PathSpline`) _asbp_spline_path))))
              (set `self.SplineIndex` 0))))
        (:`then_3`
          (bind _returnvalue_2 (`KismetSystemLibrary.K2_SetTimerDelegate` (delegate `UpdateRouteProgress`) 0.2 true))
          (set `self.RouteProgressHandler` _returnvalue_2))
        (:`then_4`
          (`self.SpawnPlayer`))))))

(event `UpdateRouteProgress`
  (if (and (> (`KismetArrayLibrary.Array_Length` (`self.PathSpline`)) 0) (== (`self.IsPaused`) false))
    (`self.UpdateRoute`)
    (`self.UpdateCompletion`)))

(event `self.ReceiveTick`
  (params (DeltaSeconds :type "Float (single-precision)"))
  (if (not (`self.IsPaused`))
    (`self.UpdateTimer` DeltaSeconds)))

(event `EnhancedInput|/Game/_Project/Blueprints/Player/Input/UI/IA_Pause`
  (params (ActionValue :type Boolean) (ElapsedSeconds :type "Float (double-precision)") (TriggeredSeconds :type "Float (double-precision)") (InputAction :type "InputAction Object Reference" :default "/Game/_Project/Blueprints/Player/Input/UI/IA_Pause.IA_Pause"))
  (:`Triggered`
    (`self.SwitchPauseState`)))

(fn `------------------------------------------------------------------`)

(fn `------------------------------------------------------------------_0`)

(fn `------------------------------------------------------------------_1`)

(fn `------------------------------------------------------------------_2`)

(fn `AddEndScreen`
  (params (`Screen Type` :type "/Game/_Project/Source/EEndScreenType Enum" :default "NewEnumerator0"))
  (bind _endscreenwidget (`self.EndScreenWidget`))
  (`/Engine/EditorBlueprintResources/StandardMacros.IsValid` _endscreenwidget
    (:`Is Valid`
      _)
    (:`Is Not Valid`
      (bind _returnvalue (`|CreateWidget` "/Game/_Project/UI/WBP_EndScreen.WBP_EndScreen_C"))
      (bind _output_get (set `self.EndScreenWidget` _returnvalue))
      (`UserWidget.AddToViewport` _output_get 0)))
  (`/Game/_Project/UI/WBP_EndScreen.SetScreen` _endscreenwidget `Screen Type`))

(fn `CallLoseProcess`
  (`self.UpdateCurrentDifficultyCompletionData` false)
  (`self.SetGamePaused` true)
  (`self.AddEndScreen` "NewEnumerator1"))

(fn `CallRestartProcess`
  (`self.RemoveEndScreen`)
  (`self.SetGamePaused` false)
  (`self.TeleportPlayerToStart`)
  (set `self.TimerValue` 0.0))

(fn `CallWinProcess`
  (switch `/Game/_Project/Source/ECompletionType` (`self.CompletionType`)
    (:`NewEnumerator0`
      (`self.SetCompletionValue` 100.0))
    (:`NewEnumerator1`
      _))
  (`self.UpdateCurrentDifficultyCompletionData` true)
  (`self.SetGamePaused` true)
  (`self.AddEndScreen` "NewEnumerator0"))

(fn `GetStartPoint`
  (returns (Transform :type "Transform Structure"))
  (return (`self.GetTransform` (`GameModeBase.K2_FindPlayerStart` (`GameplayStatics.GetGameMode`) self ""))))

(fn `RemoveEndScreen`
  (bind _endscreenwidget (`self.EndScreenWidget`))
  (`/Engine/EditorBlueprintResources/StandardMacros.IsValid` _endscreenwidget
    (:`Is Valid`
      (`Widget.RemoveFromParent` _endscreenwidget)
      (set `self.EndScreenWidget` null))))

(fn `SetCompletionValue`
  (params (Value :type "Float (double-precision)") (`Clamp Value` :type "Float (double-precision)" :default 100.0))
  (set `self.CompletionValue` (`KismetMathLibrary.FClamp` Value 0.0 `Clamp Value`))
  (set `self.CompletionValueRounded` (`KismetMathLibrary.FClamp` (`KismetMathLibrary.GridSnap_Float` Value 0.1) 0.0 `Clamp Value`)))

(fn `SetGamePaused`
  (params (Paused :type Boolean))
  (if Paused
    (`self.SetMouseCursor` true)
    (`GameplayStatics.SetGamePaused` true)
    (set `self.IsPaused` true)
    (`self.RemoveInputContext` "/Game/_Project/Blueprints/Player/Input/IMC_Gameplay.IMC_Gameplay")
    (else
      (`self.SetMouseCursor` false)
      (`GameplayStatics.SetGamePaused` false)
      (set `self.IsPaused` false)
      (`self.AddInputContext` "/Game/_Project/Blueprints/Player/Input/IMC_Gameplay.IMC_Gameplay" 2))))

(fn `SetMouseCursor`
  (params (`Show Mouse Cursor` :type Boolean))
  (bind _returnvalue (`GameplayStatics.GetPlayerController` 0))
  (bind _pausewidget (`self.PauseWidget`))
  (bind _output_get (set `PlayerController.bShowMouseCursor` `Show Mouse Cursor` (`GameplayStatics.GetPlayerController` 0)))
  (if _output_get
    (`WidgetBlueprintLibrary.SetInputMode_GameAndUIEx` _returnvalue _pausewidget "DoNotLock" false)
    (`WidgetBlueprintLibrary.SetInputMode_UIOnlyEx` _returnvalue _pausewidget :!enabledstate Disabled)
    (else
      (`WidgetBlueprintLibrary.SetInputMode_GameOnly` _returnvalue))))

(fn `SetPauseState`
  (params (`Is Paused` :type Boolean))
  (bind _pausewidget (`self.PauseWidget`))
  (`self.SetGamePaused` `Is Paused`)
  (if `Is Paused`
    (`/Engine/EditorBlueprintResources/StandardMacros.IsValid` _pausewidget
      (:`Is Not Valid`
        (bind _returnvalue (`|CreateWidget` "/Game/_Project/UI/WBP_PauseMenu.WBP_PauseMenu_C"))
        (bind _output_get (set `self.PauseWidget` _returnvalue))
        (`UserWidget.AddToViewport` _output_get 0)))
    (else
      (`/Engine/EditorBlueprintResources/StandardMacros.IsValid` _pausewidget
        (:`Is Valid`
          (`Widget.RemoveFromParent` _pausewidget)
          (set `self.PauseWidget` null))))))

(fn `SpawnPlayer`
  (bind (_transform_location _transform_rotation) (`KismetMathLibrary.BreakTransform` (`self.GetStartPoint`)))
  (bind _returnvalue (`|SpawnActorFromClass` "/Game/_Project/Blueprints/Player/Character/SubClasses/CharacterDoll_Default.CharacterDoll_Default_C" (`KismetMathLibrary.MakeTransform` _transform_location _transform_rotation) "Undefined" "MultiplyWithRoot" null null))
  (bind _output_get (set `self.PlayerInstance` _returnvalue))
  (`self.Possess` _output_get))

(fn `SwitchPauseState`
  (if (`self.IsPaused`)
    (`self.SetPauseState` false)
    (else
      (`self.SetPauseState` true))))

(fn `TeleportPlayerToStart`
  (bind (_transform_location _transform_rotation) (`KismetMathLibrary.BreakTransform` (`self.GetStartPoint`)))
  (bind _playerinstance (`self.PlayerInstance`))
  (`self.K2_TeleportTo` _playerinstance _transform_location _transform_rotation)
  (`/Game/_Project/Blueprints/Player/Character/BP_Character.ResetCharacterMovement` _playerinstance))

(fn `UpdateCompletion`
  (switch `/Game/_Project/Source/ECompletionType` (`self.CompletionType`)
    (:`NewEnumerator0`
      (`self.SetCompletionValue` (* (/ (`self.RouteCompleted` :!enabledstate Disabled) (`self.RouteLength` :!enabledstate Disabled)) 100.0) :!enabledstate Disabled))
    (:`NewEnumerator1`
      (`self.SetCompletionValue` (/ (`self.RouteCompleted` :!enabledstate Disabled) 100.0) 9999999.0 :!enabledstate Disabled))))

(fn `UpdateCurrentDifficultyCompletionData`
  (params (`Is Win` :type Boolean))
  (bind _gameinstance (`self.GameInstance`))
  (bind _timervalue (`self.TimerValue`))
  (bind _completionvaluerounded (`self.CompletionValueRounded`))
  (bind _selecteddifficulty (`/Game/_Project/Blueprints/Game/BP_GameInstance.SelectedDifficulty` _gameinstance))
  (bind (_value _time) (`/Game/_Project/Blueprints/Game/BP_GameInstance.GetDifficultyCompletionData` _gameinstance _selecteddifficulty))
  (bind _returnvalue (> _completionvaluerounded _value))
  (`/Game/_Project/Blueprints/Game/BP_GameInstance.SetDifficultyCompletionData` _gameinstance _selecteddifficulty (`KismetMathLibrary.SelectFloat` _completionvaluerounded _value _returnvalue) (`KismetMathLibrary.SelectFloat` _timervalue _time (or _returnvalue (and (== _completionvaluerounded _value) (<= _timervalue _time))))))

(fn `UpdateRoute`
  (bind _returnvalue_location (`KismetMathLibrary.BreakTransform` (`self.GetTransform` (`self.PlayerInstance`))))
  (bind _output (`|GetArrayItem` (`self.PathSpline`) (`self.SplineIndex`)))
  (bind (_fraction _remaining) (`/Game/_Project/Blueprints/LevelDesign/Elements/BP_SplinePath.GetCompletedLengthByLocation` _output _returnvalue_location))
  (bind _length (`/Game/_Project/Blueprints/LevelDesign/Elements/BP_SplinePath.GetPathLength` _output))
  (set `self.RouteLength` _length)
  (set `self.RouteCompleted` (- _length _remaining))
  (`self.SetCompletionValue` (* _fraction 100.0)))

(fn `UpdateTimer`
  (params (`Delta Seconds` :type "Float (double-precision)"))
  (if (not (`self.IsPaused`))
    (set `self.TimerValue` (+ (`self.TimerValue`) `Delta Seconds`))))

(fn `UserConstructionScript`)